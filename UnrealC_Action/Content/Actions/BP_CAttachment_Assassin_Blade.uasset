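; Attachment actor for the Assassin's blade weapon, moving it between holster and hand sockets and placing its foot hit collisions.
; On begin play it attaches to the holster socket and binds the left and right foot fist collision components to their foot sockets.
; Equip and unequip events call the parent logic, then reattach the blade to the hand or back to the holster.
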(event EventOnEquip
  (|CallParentFunction)
  (Class|CAttachment|Attachto "Hand_Assassin_Blade"))

(event EventOnUnEquip
  (|CallParentFunction)
  (Class|CAttachment|Attachto "Holster_Assassin"))

(event EventBeginPlay
  (|CallParentFunction)
  (Class|CAttachment|Attachto "Holster_Assassin")
  (Class|CAttachment|AttachtoCollision (Variables|Default|GetFist_Left_Foot) "Fist_Left_Foot")
  (Class|CAttachment|AttachtoCollision (Variables|Default|GetFist_Right_Foot) "Fist_Right_Foot"))

(fn ConstructionScript)