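; Anim notify state that switches the player character's ghost trail effect on for a span of an animation.
; On begin it casts the mesh owner to BP_CPlayer and sets its GhostTrail flag to true, and on end it clears the flag.
; It does nothing for owners that are not BP_CPlayer and only toggles the flag, without producing the trail itself.
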(fn GetNotifyName
  (return "GhostTrailState"))

(fn ReceivedNotifyBegin
  (params (MeshComp :type Skeletal%20Mesh%20Component%20Object%20Reference) (Animation :type Anim%20Sequence%20Base%20Object%20Reference) (TotalDuration :type Float%20%28single-precision%29))
  (bind _asbp_cplayer (Utilities|Casting|CastToBP_CPlayer (Components|GetOwner MeshComp)))
  (Variables|/Game/Player/BP_CPlayer.BP_CPlayer_C|SetGhostTrail _asbp_cplayer true)
  (return false))

(fn ReceivedNotifyEnd
  (params (MeshComp :type Skeletal%20Mesh%20Component%20Object%20Reference) (Animation :type Anim%20Sequence%20Base%20Object%20Reference))
  (bind _asbp_cplayer (Utilities|Casting|CastToBP_CPlayer (Components|GetOwner MeshComp)))
  (Variables|/Game/Player/BP_CPlayer.BP_CPlayer_C|SetGhostTrail _asbp_cplayer false)
  (return false))