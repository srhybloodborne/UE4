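; BP_CAttachment_Warp is the attachment Blueprint for the Warp action, carrying a Decal component.
; BeginPlay runs the parent logic, then hides the Decal.
; OnEquip and OnUnEquip only defer to the parent, while nodes that show and hide the Decal sit unconnected and never run.
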(event EventOnEquip
  (|CallParentFunction))

(event EventOnUnEquip
  (|CallParentFunction))

(event EventBeginPlay
  (|CallParentFunction)
  (Rendering|SetVisibility (Variables|Default|GetDecal) false false))

(fn ConstructionScript)