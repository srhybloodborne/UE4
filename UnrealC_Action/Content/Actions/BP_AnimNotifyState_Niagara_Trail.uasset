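; Anim notify state, shown as "Niagara Trail", that plays an attached Niagara effect for the duration of an animation window.
; On begin it spawns the effect on the mesh at a configurable socket and relative offset.
; On end it searches the owner's Niagara components and destroys the first matching both asset and socket, removing it outright rather than deactivating it.
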(fn ReceivedNotifyBegin
  (params (MeshComp :type Skeletal%20Mesh%20Component%20Object%20Reference) (Animation :type Anim%20Sequence%20Base%20Object%20Reference) (TotalDuration :type Float%20%28single-precision%29))
  (Niagara|SpawnSystemAttached (Variables|Default|GetParticleEffect) MeshComp (Variables|Default|GetSockeName) (Variables|Default|GetLoaction) (Variables|Default|GetRotation) "KeepRelativeOffset" true)
  (return false))

(fn ReceivedNotifyEnd
  (params (MeshComp :type Skeletal%20Mesh%20Component%20Object%20Reference) (Animation :type Anim%20Sequence%20Base%20Object%20Reference))
  (for _array_element (Actor|GetComponentsByClass (Components|GetOwner MeshComp) "/Script/Niagara.NiagaraComponent")
    (LocalVariables|SetParticle _array_element)
    (if (== (AssetData|GetAsset (LocalVariables|GetParticle)) (Variables|Default|GetParticleEffect))
      (if (Utilities|Name|Equal(Name) (Variables|Default|GetSockeName) (Transformation|GetAttachSocketName (LocalVariables|GetParticle)))
        (Components|DestroyComponent (LocalVariables|GetParticle) (LocalVariables|GetParticle))
        (return false)))))

(fn ReceivedNotifyTick
  (params (MeshComp :type Skeletal%20Mesh%20Component%20Object%20Reference) (Animation :type Anim%20Sequence%20Base%20Object%20Reference) (FrameDeltaTime :type Float%20%28single-precision%29))
  (return false))

(fn GetNotifyName
  (return "Niagara Trail"))