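; Ghost trail actor that leaves a frozen afterimage of a skeletal mesh's pose, then removes itself.
; Init copies the owner's current pose onto a PoseableMesh and replaces each material slot with a dynamic instance of the supplied ghost material.
; An Opacity timeline, started from Init, drives the Opacity parameter on those instances and destroys the actor when finished.
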(event Custom|Init
  (params (Owner :type Skeletal%20Mesh%20Component%20Object%20Reference) (GhostTrailMaterialInput :type Material%20Instance%20Object%20Reference))
  (Variables|Default|SetGhostTrailMaterial GhostTrailMaterialInput)
  (Class|PoseableMeshComponent|CopyPosefromSkeletalComponent (Variables|Default|GetPoseableMesh) Owner)
  (for (_ _array_index) (Rendering|Material|GetMaterials (Variables|Default|GetPoseableMesh))
    (bind _returnvalue (Rendering|Material|CreateDynamicMaterialInstance (Variables|Default|GetGhostTrailMaterial) "None" :!class /Script/Engine.KismetMaterialLibrary))
    (Utilities|FlowControl|Sequence
      (:then_0
        (Utilities|Array|Add (Variables|Default|GetMaterials) _returnvalue))
      (:then_1
        (Rendering|Material|SetMaterial (Variables|Default|GetPoseableMesh) _array_index _returnvalue))))
  (Components|Timeline|PlayfromStart (Variables|Colors|GetOpacity)))

(fn ConstructionScript)