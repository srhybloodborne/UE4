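; Player character Blueprint that adds visual feedback for getting hit, ghost trails and an outline effect.
; Tick shows a timeline-faded blood overlay widget while the State component reports hit mode, and consumes the GhostTrail flag to spawn a mesh ghost with an Assassin, Katana or Bow material.
; T toggles a timeline that expands or reverses the outline radius in a material parameter collection, centered on the mesh's location.
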(event Custom|Create%20Ghost%20Trail
  (bind _returnvalue (Game|SpawnActorfromClass "/Game/Actions/BP_GhostTrail.BP_GhostTrail_C" (Transformation|GetWorldTransform (Variables|Character|GetMesh)) "Undefined" 0 0))
  (Utilities|FlowControl|Sequence
    (:then_0
      (if (Class|CActionComponent|IsAssassinMode (Variables|Default|GetAction))
        (Default|Init _returnvalue (Variables|Character|GetMesh) "/Game/Character/Materials/MI_GhostTrail_Assassin.MI_GhostTrail_Assassin")))
    (:then_1
      (if (Class|CActionComponent|IsKatanaMode (Variables|Default|GetAction))
        (Default|Init _returnvalue (Variables|Character|GetMesh) "/Game/Character/Materials/MI_GhostTrail_Katana.MI_GhostTrail_Katana")))
    (:then_2
      (if (Class|CActionComponent|IsBowMode (Variables|Default|GetAction))
        (Default|Init _returnvalue (Variables|Character|GetMesh) "/Game/Character/Materials/MI_GhostTrail_Bow.MI_GhostTrail_Bow")))))

(event EventBeginPlay
  (|CallParentFunction)
  (bind _returnvalue (UserInterface|CreateWidget "/Game/Widgets/WB_BloodEffect.WB_BloodEffect_C"))
  (bind _output_get (Variables|Default|SetBloodEffectReference _returnvalue))
  (UserInterface|Viewport|AddtoViewport _output_get 0)
  (Widget|SetVisibility (Variables|Default|GetBloodEffectReference) "Hidden"))

(event EventTick
  (params (DeltaSeconds :type Float%20%28single-precision%29))
  (bind _bloodeffectreference (Variables|Default|GetBloodEffectReference))
  (Utilities|FlowControl|Sequence
    (:then_0
      (if (Variables|Default|GetGhostTrail)
        (CallFunction|CreateGhostTrail)
        (Variables|Default|SetGhostTrail false)))
    (:then_1
      (if (Class|CStateComponent|IsHittedMode (Variables|Default|GetState))
        (Widget|SetVisibility (Variables|Default|GetBloodEffectReference) "Visible")
        (bind _c_bloodeffect (Timeline|BloodEffect Play)
          (:Update
            (Appearance|SetColorandOpacity _bloodeffectreference (Math|Color|MakeColor 1.0 1.0 1.0 _c_bloodeffect) :!class /Script/UMG.UserWidget)))
        (else
          (Widget|SetVisibility _bloodeffectreference "Hidden"))))))

(event Input|KeyboardEvents|T
  (params (Key :type Key%20Structure :default "None"))
  ;[1 1 1] TODO
  (:Pressed
    (Rendering|Material|SetVectorParameterValue "/Game/Materials/Mine/PC_OutLine.PC_OutLine" "Position" (Math|Conversions|ToLinearColor(Vector) (Transformation|GetWorldLocation (Variables|Character|GetMesh))) :!class /Script/Engine.KismetMaterialLibrary)
    (Utilities|FlowControl|FlipFlop
      (:A
        (bind _새_트랙_0 (Timeline|타임라인_0 Play)
          (:Update
            (Rendering|Material|SetScalarParameterValue "/Game/Materials/Mine/PC_OutLine.PC_OutLine" "Radius" _새_트랙_0 :!class /Script/Engine.KismetMaterialLibrary))))
      (:B
        (Timeline|타임라인_0 Reverse)))))

(fn ConstructionScript)