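; Wizard weapon that casts through a swappable active skill, spawning Heal, Warp and Throw skill actors at BeginPlay and starting on Heal.
; Skills attach to the owning character's mesh, with Throw on the wizard hand socket.
; Attack, Attacked and selection events forward to the active skill as Spell, Spelled and focus calls, while ChangeSkill hands focus between skills.
; Attack casts when CanAttack equals the skill's validity, rather than requiring both be true.
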(event EventBeginPlay
  (|CallParentFunction)
  (Utilities|FlowControl|Sequence
    (:then_0
      (|Spawn&AttachHeal))
    (:then_1
      (|Spawn&AttachWarp))
    (:then_2
      (|Spawn&AttachThrow))
    (:then_3
      (CallFunction|ChangeSkill (Variables|Default|GetHeal)))))

(event EventOnSelected
  (bind _skill (Variables|Default|GetSkill))
  (|CallParentFunction)
  (Utilities|IsValid _skill
    (:Is%20Valid
      (Default|OnFocus _skill))))

(event EventOffSelected
  (bind _skill (Variables|Default|GetSkill))
  (|CallParentFunction)
  (Utilities|IsValid _skill
    (:Is%20Valid
      (Default|OffFocus _skill))))

(event EventAttack
  (|CallParentFunction)
  (if (Math|Boolean|Equal(Boolean) (CallFunction|CanAttack) (Utilities|IsValid (Variables|Default|GetSkill)))
    (CallFunction|SetStateSeplling)
    (Default|Spell (Variables|Default|GetSkill))))

(event EventAttacked
  (|CallParentFunction)
  (Default|Spelled (Variables|Default|GetSkill)))

(fn ConstructionScript
  (|CallParentFunction))

(fn ChangeSkill
  (params (NewSkill :type BP%20Skill%20Object%20Reference))
  (if (!= NewSkill (Variables|Default|GetSkill))
    (Utilities|IsValid (Variables|Default|GetSkill)
      (:Is%20Valid
        (Default|OffFocus (Variables|Default|GetSkill)))
      (:Is%20Not%20Valid
        _))
    (Utilities|IsValid NewSkill
      (:Is%20Valid
        (bind _output_get (Variables|Default|SetSkill NewSkill))
        (Default|OnFocus _output_get))
      (:Is%20Not%20Valid
        (Variables|Default|SetSkill 0)))))