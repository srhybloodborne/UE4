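; Wizard healing skill that restores a fixed amount of the caster's health.
; It extends a parent skill's Spell and Spelled events, calling the parent logic first in each.
; Spell disables the wizard's movement and plays the heal montage.
; Spelled re-enables movement and increases health through the character's status component.
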(event EventSpell
  ;[1 1 1] Spell
  (|CallParentFunction)
  (Default|SetStateMove (CallFunction|GetWizard) false)
  (Animation|PlayAnimMontage (CallFunction|GetWizardCharacter) "/Game/Character/Montages/MG_Heal_Montage.MG_Heal_Montage" 1.0 "None"))

(event EventSpelled
  ;[1 1 1] Spelled
  (|CallParentFunction)
  (Class|IState|SetStateMove(Message) (CallFunction|GetWizard) true)
  (Default|IncreasceHealth (Actor|GetComponentbyClass (CallFunction|GetWizardCharacter) "/Game/Components/StatusCompoent.StatusCompoent_C") 2e+01))

(fn ConstructionScript
  (|CallParentFunction))