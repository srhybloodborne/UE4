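; BP_ThrowItem is a thrown item for the Wizard's throw skill that destroys itself after a short lifespan.
; Helper functions cast up the owner chain to BP_Skill_Throw, then BP_Wizard.
; BeginOverlap ignores the Wizard's owner, routes damage to other actors through BP_Wizard, spawns an explosion emitter and destroys the item.
; No event here calls BeginOverlap; its caller supplies the actor, effect and damage.
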(event EventBeginPlay
  (Actor|SetLifeSpan 2.0))

(fn ConstructionScript)

(fn GetOwnertoThrow
  (bind _asbp_skill_throw (Utilities|Casting|CastToBP_Skill_Throw (Components|GetOwner)))
  (return _asbp_skill_throw))

(fn GetOwnertoWizard
  (bind _asbp_wizard (Utilities|Casting|CastToBP_Wizard (Components|GetOwner (CallFunction|GetOwnertoThrow))))
  (return _asbp_wizard))

(fn BeginOverlap
  (params (OhterActor :type Actor%20Object%20Reference) (Explosion :type Particle%20System%20Object%20Reference) (Damage :type Float%20%28single-precision%29) (Location :type Vector) (Scale :type Vector :default "1.000000,1.000000,1.000000"))
  (if (!= OhterActor (Components|GetOwner (CallFunction|GetOwnertoWizard)))
    (Default|SendDamage (CallFunction|GetOwnertoWizard) Damage OhterActor)
    (Effects|SpawnEmitteratLocation Explosion (+ (Transformation|GetActorLocation OhterActor) Location) "0, 0, 0" Scale)
    (Actor|DestroyActor)))