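; Wizard warp skill that teleports the character to the floor point under the mouse cursor.
; While focused, Tick shows a target marker wherever a cursor trace hits a WorldStatic actor with "Floor" in its display name.
; Spell stores that point, locks movement and plays the warp montage, or calls the wizard's Attacked on an invalid target.
; A separate Warp event performs the teleport, and Spelled restores movement.
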(event Custom|Warp
  ;[1 1 1] Warp : 실제로 Actor를 이동시킴
  (if (Variables|Default|GetWarpable)
    (Variables|Default|SetWarpable false)
    (Transformation|SetActorLocation (CallFunction|GetWizardCharacter) (Variables|Default|GetLocation) false true)))

(event EventTick
  (params (DeltaSeconds :type Float%20%28single-precision%29))
  (bind _cursor (Variables|Default|GetCursor))
  ;[1 1 1] Tick Event : Warp Cursor 표시
  (bind _location (Utilities|GetCursorLocation)
    (:True
      (Transformation|SetWorldLocation _cursor _location false false)
      (if (Variables|Default|GetFocus)
        (Rendering|SetVisibility (Variables|Default|GetCursor) true false)
        (else
          (Rendering|SetVisibility (Variables|Default|GetCursor) false false))))
    (:False
      (Rendering|SetVisibility _cursor false false))))

(event EventBeginPlay
  (|CallParentFunction))

(event EventOnFocus
  (|CallParentFunction)
  (Variables|Default|SetFocus true))

(event EventOffFocus
  (|CallParentFunction)
  (Variables|Default|SetFocus false))

(event EventSpell
  ;[1 1 1] Spell
  (|CallParentFunction)
  (bind _location (Utilities|GetCursorLocation)
    (:True
      (Variables|Default|SetLocation _location)
      (Variables|Default|SetWarpable true)
      (Default|SetStateMove (CallFunction|GetWizard) false)
      (Animation|PlayAnimMontage (CallFunction|GetWizardCharacter) "/Game/Character/Montages/MG_Warp_Montage.MG_Warp_Montage" 1.0 "None"))
    (:False
      (Default|Attacked (CallFunction|GetWizard))
      (Variables|Default|SetWarpable false))))

(event EventSpelled
  ;[1 1 1] Spelled
  (|CallParentFunction)
  (Class|IState|SetStateMove(Message) (CallFunction|GetWizard) true))

(fn ConstructionScript
  (|CallParentFunction))