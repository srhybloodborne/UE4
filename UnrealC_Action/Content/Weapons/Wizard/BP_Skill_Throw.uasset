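; Wizard throw skill that plays a throw montage on cast and spawns the currently selected throw-item actor from the character's hand.
; An array of throw-item structs pairs each actor class with an attach particle, and ChangeItem selects an entry by class and swaps the particle.
; The particle shows only while the skill has focus.
; Throw spawns the item at the hand socket, using the character's yaw with a slight offset.
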(event Custom|Throw
  (bind _ascharacter (CallFunction|GetWizardCharacter))
  ;[1 1 1] Throw : Actor(BP_ThrowItem_xxxxx)
  (Game|SpawnActorfromClass (.ThrowItemClass (Utilities|Struct|BreakFThrowItem (Utilities|Array|Get(acopy) (Variables|Default|GetThrowItems) (Variables|Default|GetCurrentItem_Index)))) (Math|Transform|MakeTransform (Transformation|GetSocketLocation (Variables|/Script/Engine.Character|GetMesh _ascharacter) "Hand_ThrowItem") (Math|Rotator|MakeRotator 0.0 0.0 (- (.yaw (Transformation|GetActorRotation _ascharacter)) 5.0)) "0.500000,0.500000,0.500000") "Undefined" self 0))

(event EventBeginPlay
  ;[1 1 1] BeginPlay Event : 구조체 데이터에 따른 한손에 파티클 시스템 Set
  (Effects|Components|ParticleSystem|SetTemplate (Variables|Default|GetParticleSystem) (.AttachParticle (Utilities|Struct|BreakFThrowItem (Utilities|Array|Get(acopy) (Variables|Default|GetThrowItems) (Variables|Default|GetCurrentItem_Index)))))
  (Rendering|SetVisibility (Variables|Default|GetParticleSystem) false false))

(event EventOnFocus
  (|CallParentFunction)
  (Rendering|SetVisibility (Variables|Default|GetParticleSystem) true false))

(event EventOffFocus
  (|CallParentFunction)
  (Rendering|SetVisibility (Variables|Default|GetParticleSystem) false false))

(event EventSpell
  ;[1 1 1] Spell : Motion
  (|CallParentFunction)
  (Animation|PlayAnimMontage (CallFunction|GetWizardCharacter) "/Game/Character/Montages/MG_Throw_Montage.MG_Throw_Montage" 1.0 "None"))

(event EventSpelled
  ;[1 1 1] Spelled
  (|CallParentFunction)
  (Class|IState|SetStateMove(Message) (CallFunction|GetWizard) true))

(fn ConstructionScript
  (|CallParentFunction))

(fn ChangeItem
  (params (NewClass :type BP%20Throw%20Item%20Class%20Reference))
  (bind _array_index (Utilities|Array|ForEachLoopwithBreak (Variables|Default|GetThrowItems) :!label _label)
    (:LoopBody
      (LocalVariables|SetFindIndex _array_index)
      (if (== (.ThrowItemClass (Utilities|Struct|BreakFThrowItem (Utilities|Array|Get(acopy) (Variables|Default|GetThrowItems) _array_index))) NewClass)
        (goto _label Break)))
    (:Completed
      (bind _output_get (Variables|Default|SetCurrentItem_Index (LocalVariables|GetFindIndex)))
      (Effects|Components|ParticleSystem|SetTemplate (Variables|Default|GetParticleSystem) (.AttachParticle (Utilities|Struct|BreakFThrowItem (Utilities|Array|Get(acopy) (Variables|Default|GetThrowItems) _output_get)))))))