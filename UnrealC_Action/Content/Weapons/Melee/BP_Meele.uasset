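; BP_Meele is a melee weapon Blueprint that runs montage-based combo attacks on its owning Character.
; BeginPlay caches DataTable rows matching its MeleeType, each setting a combo step's montage, playback and movement permission.
; Attack starts the combo or, while EnableNextCombo is open, queues the next step for PlayNextCombo; Attacked resets it.
; SendDamage hits each actor once until OffCollision clears HittedActors; OnCollision, StartCombo and EndCombo are empty hooks.
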(event Custom|PlayNextCombo
  ;[1 1 1] Play Next Combo
  (if (Variables|Default|GetExistNextCombo)
    (Variables|Default|SetExistNextCombo false)
    (CallFunction|PlayComboMontage)
    (Variables|Default|SetLastCombo (== (Variables|Default|GetComboCount) (- (Utilities|Array|Length (Variables|Default|GetMeeleDatas)) 1)))))

(event EventBeginPlay
  ;[1 1 1] Begin Play
  (|CallParentFunction)
  (bind _outrownames (DataTable|GetDataTableRowNames (Variables|Default|GetDataTable)))
  (for _array_element _outrownames
    (bind _returnvalue (Utilities|GetDataTableRow (Variables|Default|GetDataTable) _array_element)
      (:then
        (if (Utilities|Enum|Equal(Enum) (.Type (Utilities|Struct|BreakFMeeleData _returnvalue)) (Variables|Default|GetMeleeType))
          (Utilities|Array|Add (Variables|Default|GetMeeleDatas) _returnvalue))))))

(event EventAttacked
  ;[1 1 1] Attacked
  (|CallParentFunction)
  (CallFunction|SetStateMove true)
  (Variables|Default|SetComboCount 0)
  (Variables|Default|SetExistNextCombo false)
  (Variables|Default|SetLastCombo false)
  (CallFunction|EndCombo))

(event EventAttack
  ;[1 1 1] Attack
  (|CallParentFunction)
  (if (Variables|Default|GetEnableNextCombo)
    (Math|Integer|IncrementInt (Variables|Default|GetComboCount)
      (:%20%20
        (Variables|Default|SetEnableNextCombo false)
        (Variables|Default|SetExistNextCombo true)))
    (elif (CallFunction|CanAttack)
      (CallFunction|SetStateAttacking)
      (CallFunction|PlayComboMontage)
      (CallFunction|StartCombo))))

(fn ConstructionScript
  (|CallParentFunction))

(fn PlayComboMontage
  (bind _meeledatas (Variables|Default|GetMeeleDatas))
  (bind _combocount (Variables|Default|GetComboCount))
  (bind _output (Utilities|Array|Get(acopy) _meeledatas _combocount))
  (bind _ascharacter (Utilities|Casting|CastToCharacter (Components|GetOwner)))
  (Animation|PlayAnimMontage _ascharacter (.montage _output) (.playrate _output) (.startsectionname _output))
  (CallFunction|SetStateMove (.canmove _output)))

(fn OnCollision
  (params (CollisionType :type E_CollisionType%20Enum :default "NewEnumerator4")))

(fn OffCollision
  (Utilities|Array|Clear (Variables|Default|GetHittedActors)))

(fn SendDamage
  (params (Damage :type Float%20%28single-precision%29) (OtherActor :type Actor%20Object%20Reference))
  ;[1 1 1] 연타검사후 Send Damage
  (bind _array_element (Utilities|Array|ForEachLoopwithBreak (Variables|Default|GetHittedActors) :!label _label)
    (:LoopBody
      (if (== _array_element OtherActor)
        (LocalVariables|SetFindActor (== _array_element OtherActor))
        (goto _label Break)))
    (:Completed
      (if (not (LocalVariables|GetFindActor))
        (Utilities|Array|Add (Variables|Default|GetHittedActors) OtherActor)
        (bind _result (|CallParentFunction Damage OtherActor))
        (return _result)))))

(fn StartCombo)

(fn EndCombo)