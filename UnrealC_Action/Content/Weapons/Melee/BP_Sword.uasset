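; Melee sword weapon Blueprint that deals combo-scaled damage through a capsule hitbox.
; The capsule starts without collision and is switched on and off by overrides of the parent's OnCollision and OffCollision events.
; On overlap it gets the current combo's power from WeaponPowerComponent and sends it as damage to the overlapped actor.
; Combo start and end notify that component, and PlayLastCombo spawns a lightning particle effect at a given location and scale.
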(event OnComponentBeginOverlap(Capsule)
  (params (OverlappedComponent :type Primitive%20Component%20Object%20Reference) (OtherActor :type Actor%20Object%20Reference) (OtherComp :type Primitive%20Component%20Object%20Reference) (OtherBodyIndex :type Integer) (bFromSweep :type Boolean) (SweepResult :type Hit%20Result%20Structure%20%28by%20ref%29))
  (bind _attack (Default|GetComboPower (Variables|Default|GetWeaponPowerComponent) (Variables|Default|GetComboCount)))
  (CallFunction|SendDamage _attack OtherActor))

(event Custom|Play%20Last%20Combo
  (params (Location :type Vector) (Scale :type Vector :default "1.000000,1.000000,1.000000"))
  (Effects|SpawnEmitteratLocation "/Game/Particles/P_Lightning.P_Lightning" Location "0, 0, 0" Scale))

(event EventOnCollision
  (params (CollisionType :type E_CollisionType%20Enum :default "NewEnumerator4"))
  (|CallParentFunction CollisionType)
  (Collision|SetCollisionEnabled (Variables|Default|GetCapsule) "QueryAndPhysics"))

(event EventOffCollision
  (|CallParentFunction)
  (Collision|SetCollisionEnabled (Variables|Default|GetCapsule) "NoCollision"))

(event EventBeginPlay
  (|CallParentFunction)
  (Collision|SetCollisionEnabled (Variables|Default|GetCapsule) "NoCollision"))

(event EventStartCombo
  (Default|StartAttack (Variables|Default|GetWeaponPowerComponent)))

(event EventEndCombo
  (Default|EndAttack (Variables|Default|GetWeaponPowerComponent)))

(fn ConstructionScript)