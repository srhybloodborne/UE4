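; Unarmed melee weapon that turns the owning character's hands and feet into hit volumes.
; On BeginPlay, four sphere components attach to fist sockets on the owner's mesh and start with collision off.
; OnCollision enables the sphere matching the requested limb, and OffCollision disables all spheres; overlaps send damage to the other actor.
; StartCombo and EndCombo start and end attacks on the WeaponPowerComponent.
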(event OnComponentBeginOverlap(RightFoot)
  (params (OverlappedComponent :type Primitive%20Component%20Object%20Reference) (OtherActor :type Actor%20Object%20Reference) (OtherComp :type Primitive%20Component%20Object%20Reference) (OtherBodyIndex :type Integer) (bFromSweep :type Boolean) (SweepResult :type Hit%20Result%20Structure%20%28by%20ref%29))
  ;[1 1 1] 노가다라 칼만함
  (CallFunction|SendDamage (Variables|Default|GetDamage) OtherActor))

(event OnComponentBeginOverlap(LeftFoot)
  (params (OverlappedComponent :type Primitive%20Component%20Object%20Reference) (OtherActor :type Actor%20Object%20Reference) (OtherComp :type Primitive%20Component%20Object%20Reference) (OtherBodyIndex :type Integer) (bFromSweep :type Boolean) (SweepResult :type Hit%20Result%20Structure%20%28by%20ref%29))
  ;[1 1 1] 노가다라 칼만함
  (CallFunction|SendDamage (Variables|Default|GetDamage) OtherActor))

(event OnComponentBeginOverlap(RightHand)
  (params (OverlappedComponent :type Primitive%20Component%20Object%20Reference) (OtherActor :type Actor%20Object%20Reference) (OtherComp :type Primitive%20Component%20Object%20Reference) (OtherBodyIndex :type Integer) (bFromSweep :type Boolean) (SweepResult :type Hit%20Result%20Structure%20%28by%20ref%29))
  ;[1 1 1] 노가다라 칼만함
  (CallFunction|SendDamage (Variables|Default|GetDamage) OtherActor))

(event OnComponentBeginOverlap(LeftHand)
  (params (OverlappedComponent :type Primitive%20Component%20Object%20Reference) (OtherActor :type Actor%20Object%20Reference) (OtherComp :type Primitive%20Component%20Object%20Reference) (OtherBodyIndex :type Integer) (bFromSweep :type Boolean) (SweepResult :type Hit%20Result%20Structure%20%28by%20ref%29))
  ;[1 1 1] 노가다라 칼만함
  (CallFunction|SendDamage (Variables|Default|GetDamage) OtherActor))

(event EventOnCollision
  (params (CollisionType :type E_CollisionType%20Enum :default "NewEnumerator4"))
  (|CallParentFunction CollisionType)
  (switch Utilities|FlowControl|Switch|SwitchonE_CollisionType CollisionType
    (:NewEnumerator0
      (Collision|SetCollisionEnabled (Variables|Default|GetLeftHand) "QueryAndPhysics"))
    (:NewEnumerator1
      (Collision|SetCollisionEnabled (Variables|Default|GetRightHand) "QueryAndPhysics"))
    (:NewEnumerator2
      (Collision|SetCollisionEnabled (Variables|Default|GetLeftFoot) "QueryAndPhysics"))
    (:NewEnumerator3
      (Collision|SetCollisionEnabled (Variables|Default|GetRightFoot) "QueryAndPhysics"))))

(event EventOffCollision
  (|CallParentFunction)
  (CallFunction|SetCollision "NoCollision"))

(event EventStartCombo
  (Default|StartAttack (Variables|Default|GetWeaponPowerComponent)))

(event EventBeginPlay
  (|CallParentFunction)
  (CallFunction|AttachtoSocket (Variables|Default|GetLeftHand) "Fist_Left_Hand")
  (CallFunction|AttachtoSocket (Variables|Default|GetRightHand) "Fist_Right_Hand")
  (CallFunction|AttachtoSocket (Variables|Default|GetLeftFoot) "Fist_Left_Foot")
  (CallFunction|AttachtoSocket (Variables|Default|GetRightFoot) "Fist_Right_Foot")
  (CallFunction|SetCollision "NoCollision"))

(event EventEndCombo
  (Default|EndAttack (Variables|Default|GetWeaponPowerComponent)))

(fn ConstructionScript)

(fn AttachtoSocket
  (params (Sphere :type Sphere%20Component%20Object%20Reference) (SocketName :type Name))
  (bind _ascharacter (Utilities|Casting|CastToCharacter (Components|GetOwner)))
  (Transformation|AttachComponentToComponent Sphere (Variables|/Script/Engine.Character|GetMesh _ascharacter) SocketName "KeepRelative" "KeepRelative" "KeepRelative" true))

(fn SetCollision
  (params (CollisionEnabled :type ECollisionEnabled%20Enum :default "NoCollision"))
  (for _array_element (Actor|GetComponentsByClass "/Script/Engine.SphereComponent")
    (Collision|SetCollisionEnabled _array_element CollisionEnabled)))